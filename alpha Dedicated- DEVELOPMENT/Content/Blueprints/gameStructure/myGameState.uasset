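; Game State Blueprint that runs a server-authoritative chat system with Global and Clan channels.
; Channel structs hold messages and listening player controllers, and are created on first post or watch.
; New messages notify listeners through BPI_chatSystemChannelListener with the channel's full message list.
; Clan channels require a positive ClanID, but lookup leaves the ID comparison unwired, so all clans match the first Clan channel.
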(event EventSendChatMessage
  (params (channel :type E_ChatSystemChannels%20Enum) (clanID :type Integer) (message :type S%20Channel%20Message%20Structure))
  (Networking|SwitchHasAuthority
    (:Authority
      (chatSystem|AddChannelMessage channel clanID message))))

(event EventWatchChatChannel
  (params (channel :type E_ChatSystemChannels%20Enum :default "NewEnumerator0") (clanID :type Integer) (playerController :type Player%20Controller%20Object%20Reference))
  (Networking|SwitchHasAuthority
    (:Authority
      (chatSystem|AddChannelListener channel clanID playerController))))

(fn ConstructionScript)

(fn AddChannelMessage
  (params (channel :type E_ChatSystemChannels%20Enum) (clanID :type Integer) (message :type S%20Channel%20Message%20Structure))
  (Networking|SwitchHasAuthority
    (:Authority
      (LocalVariables|SettheMessage message)
      (LocalVariables|SettheChannel channel)
      (LocalVariables|SettheClanID clanID)
      (switch Utilities|FlowControl|Switch|SwitchonE_ChatSystemChannels (LocalVariables|GettheChannel)
        (:NewEnumerator0
          (bind (_ischannelfound _index _messagechannel) (chatSystem|FindMessageChannel (LocalVariables|GettheChannel) (LocalVariables|GettheClanID) :!label _label))
          (LocalVariables|SetmessageChannel _messagechannel)
          (LocalVariables|SetchannelIndex _index)
          (if _ischannelfound
            ;[0 0.1655 1] add message to the existing channel
            (Utilities|Array|Add (Utilities|Struct|BreakS_channel (LocalVariables|GetmessageChannel)) (LocalVariables|GettheMessage))
            (bind _structout (Utilities|Struct|SetmembersinS_channel (LocalVariables|GetmessageChannel) (Utilities|Struct|BreakS_channel (LocalVariables|GetmessageChannel))))
            (Utilities|Array|SetArrayElem (Variables|ChatSystem|GetchannelMessages) (LocalVariables|GetchannelIndex) _structout)
            (else
              ;[0 0.1655 1] create message channel if it doesnt exist yet
              (bind _structout_2 (Utilities|Struct|SetmembersinS_channel (ChatSystem|CreateMessageChannel (LocalVariables|GettheChannel) (LocalVariables|GettheClanID)) (Utilities|Array|MakeArray (LocalVariables|GettheMessage))))
              (bind _output_get (LocalVariables|SetmessageChannel _structout_2))
              (Utilities|Array|Add (Variables|ChatSystem|GetchannelMessages) _output_get)))
          ;[0 1 0.08737] notify channel listeners that a new message arrived
          (chatSystem|NotifyChannelUpdated (LocalVariables|GetmessageChannel)))
        (:NewEnumerator1
          ;[0 0.3448 0.965] check player is in guild
          (if (> (LocalVariables|GettheClanID) 0)
            (goto _label)))))))

(fn FindMessageChannel
  (params (channel :type E_ChatSystemChannels%20Enum) (clanID :type Integer))
  (bind (_index _messagechannel) (chatSystem|IsMessageChannelCreated channel clanID))
  (if (== _index -1)
    (return false -1 "")
    (else
      (return true _index _messagechannel))))

(fn IsMessageChannelCreated
  (params (channel :type E_ChatSystemChannels%20Enum) (clanID :type Integer))
  (Networking|SwitchHasAuthority
    (:Authority
      (LocalVariables|SettheChannel channel)
      (LocalVariables|SettheClanID clanID)
      (for (_array_element _array_index) (Variables|ChatSystem|GetchannelMessages)
        (LocalVariables|SettheFoundChannel _array_element)
        (LocalVariables|SettheChannelIndex _array_index)
        (if (Utilities|Enum|Equal(Enum) (.channel (Utilities|Struct|BreakS_channel _array_element)) (LocalVariables|GettheChannel))
          (switch Utilities|FlowControl|Switch|SwitchonE_ChatSystemChannels (LocalVariables|GettheChannel)
            (:NewEnumerator0
              ;[0 0.3448 0.965] global chat
              (return (LocalVariables|GettheChannelIndex) (LocalVariables|GettheFoundChannel)))
            (:NewEnumerator1
              ;[0 0.3448 0.965] check that the clan ID are matching
              (if true
                (return (LocalVariables|GettheChannelIndex) (LocalVariables|GettheFoundChannel)))))))
      (return -1 ""))))

(fn NotifyChannelUpdated
  (params (channel :type S%20Channel%20Structure))
  (bind (_channel _messages _playercontrollers) (Utilities|Struct|BreakS_channel channel))
  (Networking|SwitchHasAuthority
    (:Authority
      (LocalVariables|SettheChannel _channel)
      (LocalVariables|Setmessages _messages)
      ;[0 0.1655 1] notify each channel listener with an updated list of messages
      (for _array_element _playercontrollers
        (bind _asbpi_chat_system_channel_listener (Utilities|Casting|CastToBPI_chatSystemChannelListener _array_element))
        (Default|OnChatChannelUpdated _asbpi_chat_system_channel_listener (LocalVariables|GettheChannel) (LocalVariables|Getmessages))))))

(fn AddChannelListener
  (params (channel :type E_ChatSystemChannels%20Enum) (clanID :type Integer) (playerController :type Player%20Controller%20Object%20Reference))
  (Networking|SwitchHasAuthority
    (:Authority
      (LocalVariables|SettheChannel channel)
      (LocalVariables|Setplayer playerController)
      (LocalVariables|SettheClanID clanID)
      (switch Utilities|FlowControl|Switch|SwitchonE_ChatSystemChannels (LocalVariables|GettheChannel)
        (:NewEnumerator0
          (bind (_ischannelfound _index _messagechannel) (chatSystem|FindMessageChannel (LocalVariables|GettheChannel) (LocalVariables|GettheClanID) :!label _label))
          (LocalVariables|SetmessageChannel _messagechannel)
          (LocalVariables|SetchannelIndex _index)
          ;[0 0.1655 1] add player to existing channel
          (if _ischannelfound
            (bind _output_get (LocalVariables|SetnotifyList (Utilities|Struct|BreakS_channel (LocalVariables|GetmessageChannel))))
            (if (not (> (Utilities|Array|FindItem _output_get (LocalVariables|Getplayer)) -1))
              (Utilities|Array|Add _output_get (LocalVariables|Getplayer))
              (bind _structout (Utilities|Struct|SetmembersinS_channel (LocalVariables|GetmessageChannel) (LocalVariables|GetnotifyList)))
              (Utilities|Array|SetArrayElem (Variables|ChatSystem|GetchannelMessages) (LocalVariables|GetchannelIndex) _structout))
            (else
              ;[0 0.1655 1] channel  doesnt exist so create it
              (bind _structout_2 (Utilities|Struct|SetmembersinS_channel (ChatSystem|CreateMessageChannel (LocalVariables|GettheChannel) (LocalVariables|GettheClanID)) (Utilities|Array|MakeArray (LocalVariables|Getplayer))))
              (Utilities|Array|Add (Variables|ChatSystem|GetchannelMessages) _structout_2))))
        (:NewEnumerator1
          ;[0 0.3448 0.965] check player is in a clan
          (if (> (LocalVariables|GettheClanID) 0)
            (goto _label)))))))

(fn GetChatSystem
  (bind _asbpi_chat_system (Utilities|Casting|CastToBPI_ChatSystem self)
    (:then
      (return _asbpi_chat_system))
    (:CastFailed
      (return 0))))

(fn CreateMessageChannel
  (params (channel :type E_ChatSystemChannels%20Enum) (clanID :type Integer))
  (LocalVariables|SettheChannel channel)
  (LocalVariables|SettheClanID clanID)
  (switch Utilities|FlowControl|Switch|SwitchonE_ChatSystemChannels (LocalVariables|GettheChannel)
    (:NewEnumerator0
      (return (Utilities|Struct|MakeS_channel (LocalVariables|GettheChannel))))
    (:NewEnumerator1
      (return (Utilities|Struct|MakeS_channel (LocalVariables|GettheChannel) (LocalVariables|GettheClanID))))))

(fn GetChatChannelMessages
  (params (channel :type E_ChatSystemChannels%20Enum :default "NewEnumerator0") (clanID :type Integer))
  (bind (_index _messagechannel) (chatSystem|IsMessageChannelCreated channel clanID))
  (Networking|SwitchHasAuthority
    (:Authority
      (if (> _index -1)
        (return true (Utilities|Struct|BreakS_channel _messagechannel))
        (else
          (return false (Utilities|Array|MakeArray)))))))