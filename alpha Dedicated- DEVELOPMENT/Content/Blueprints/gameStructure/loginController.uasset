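; Player controller for the login stage that sets up the display and shows the login screen.
; On BeginPlay it applies the desktop resolution in windowed mode, then creates the login widget and stores it on the game instance.
; It enables game-and-UI input with a locked, visible cursor.
; Releasing the Enter key action calls ShowLoginScreen on the stored widget.
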(event Custom|setupLoginScreen
  ;[0.2359 0.6483 1] create the login screen widget and add it to viewport
  (CallFunction|SetupScreenResolution)
  (CallFunction|CreateLoginWidget))

(event EventBeginPlay
  ;[0.2359 0.6483 1] create the login screen widget and add it to viewport
  (Networking|SwitchHasAuthority
    (:Authority
      _)
    (:Remote
      _))
  (CallFunction|SetupLoginScreen))

(event Input|ActionEvents|InputActionenterKeyPress
  (params (Key :type Key%20Structure :default "AnyKey"))
  (:Released
    (Default|ShowLoginScreen (Variables|/Game/Blueprints/gameStructure/myGameInstance.myGameInstance_C|GetloginWidgetRef (Utilities|GetGameInstance)))))

(fn ConstructionScript)

(fn SetupScreenResolution
  (bind _returnvalue (Settings|GetGameUserSettings))
  (Class|GameUserSettings|SetScreenResolution _returnvalue (Class|GameUserSettings|GetDesktopResolution _returnvalue))
  (Class|GameUserSettings|ApplyResolutionSettings _returnvalue false)
  (Class|GameUserSettings|SetFullscreenMode _returnvalue "Windowed")
  (Class|GameUserSettings|ApplySettings _returnvalue false))

(fn CreateLoginWidget
  (bind _returnvalue (UserInterface|CreateWidget "/Game/Blueprints/widget/loginWidget.loginWidget_C" self))
  (bind _output_get (Variables|/Game/Blueprints/gameStructure/myGameInstance.myGameInstance_C|SetloginWidgetRef (Utilities|GetGameInstance) _returnvalue))
  (UserInterface|Viewport|AddtoViewport _output_get 0)
  (Input|SetInputModeGameandUI self 0 "LockAlways" false)
  (Variables|/Script/Engine.PlayerController|SetbShowMouseCursor self true))