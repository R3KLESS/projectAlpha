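; Lobby game mode that tracks the online player count and announces departures.
; On login and logout it writes the current player count to NumberOfPlayersOnline on myGameState.
; On logout it also reads the leaving player's profile name from MyplayerState.
; It then loops over the PlayerArray indices, fetching each lobbyController by player index to call SendLogoutMessage with that name.
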(event EventPostLogin
  (params (NewPlayer :type Player%20Controller%20Object%20Reference))
  ;[0 0.3448 0.965] display how many people are online when we log in
  (bind _returnvalue (Class|GameModeBase|GetNumPlayers))
  (bind _asmy_game_state (Utilities|Casting|CastTomyGameState (Game|GetGameState)))
  (Variables|/Game/Blueprints/gameStructure/myGameState.myGameState_C|SetNumberOfPlayersOnline _asmy_game_state _returnvalue))

(event EventOnLogout
  (params (ExitingController :type Controller%20Object%20Reference))
  ;[0 0.3448 0.965] display how many people are online when we log out
  (bind _returnvalue (Class|GameModeBase|GetNumPlayers))
  (bind _asmy_game_state (Utilities|Casting|CastTomyGameState (Game|GetGameState)))
  (Variables|/Game/Blueprints/gameStructure/myGameState.myGameState_C|SetNumberOfPlayersOnline _asmy_game_state _returnvalue)
  (bind _asmyplayer_state (Utilities|Casting|CastToMyplayerState (Variables|/Script/Engine.Controller|GetPlayerState ExitingController)))
  (for (_ _array_index) (Variables|/Script/Engine.GameStateBase|GetPlayerArray (Game|GetGameState))
    (bind _aslobby_controller (Utilities|Casting|CastTolobbyController (Game|GetPlayerController _array_index)))
    (Default|SendLogoutMessage _aslobby_controller (Utilities|String|ToString(Text) (Variables|/Game/Blueprints/gameStructure/MyplayerState.MyplayerState_C|GetplayerProfileName _asmyplayer_state)))))

(fn ConstructionScript)