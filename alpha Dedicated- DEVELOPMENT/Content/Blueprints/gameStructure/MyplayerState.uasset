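; Player state that handles account registration, activation, login and profile loading through JSON POST requests to PHP scripts on the game instance's host.
; SendRequest builds each request by type, and completion routes to response handlers that update the login widget.
; Successful login stores session key and user ID, then chains into profile loading and lobby entry.
; Registration generates a random account ID client-side; the server-status check for lobby restarts sits on unreached test wiring.
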(event Custom|result
  (params (Request :type Va%20Rest%20Request%20JSON%20Object%20Reference))
  ;[0.2359 0.6483 1] working test of getting a json responce  and restarting lobby
  (bind _returnvalue (Class|VaRestRequestJSON|GetResponseObject Request))
  (bind _returnvalue_2 (Class|VaRestJsonObject|GetObjectArrayField _returnvalue "ServerQueryResults"))
  (bind _output_get (Variables|Default|SetserverQueryResultObject1 (Utilities|Array|Get(acopy) _returnvalue_2)))
  (Variables|Default|SetserverQueryResultObject2 (Utilities|Array|Get(acopy) _returnvalue_2 1))
  (if (and (Utilities|Enum|Equal(Enum) (Class|VaRestJsonObject|GetStringField _output_get "serverStatus") "offline") (Utilities|Enum|Equal(Enum) (Class|VaRestJsonObject|GetStringField _output_get "serverName") "lobby"))
    (Development|PrintString "lobby is offline . attempting to restart" true true "(R=0.000000,G=0.660000,B=1.000000,A=1.000000)" 1e+03)
    (CallFunction|RestartLobby)))

(event Custom|onRequestComplete
  (params (Request :type Va%20Rest%20Request%20JSON%20Object%20Reference))
  ;[0.4601 1 0.07955] handle responces
  (switch Utilities|FlowControl|Switch|SwitchonrequestType (Variables|Default|GetrequestType)
    (:NewEnumerator2
      (CallFunction|OnResponceLogin))
    (:NewEnumerator3
      (CallFunction|OnResponceRegistration))
    (:NewEnumerator4
      (CallFunction|OnResponceActivation))
    (:NewEnumerator7
      (CallFunction|OnResponseLoadProfile))))

(event Custom|restartLobby
  ;[0.2359 0.6483 1] working test of getting a json responce  and restarting lobby
  (Variables|Default|SetsentRequest (Class|VaRestRequestJSON|ConstructRequestExt "POST" "json"))
  (bind _output_get (Variables|Default|SetrequestType "NewEnumerator5"))
  (switch Utilities|FlowControl|Switch|SwitchonrequestType _output_get
    (:NewEnumerator5
      (CallFunction|CreateServerRequest))))

(event Custom|sendRequest
  (params (requestType :type requestType%20Enum))
  ;[0.2359 0.6483 1] send requests
  (Variables|Default|SetsentRequest (Class|VaRestRequestJSON|ConstructRequestExt "POST" "json"))
  (bind _output_get (Variables|Default|SetrequestType requestType))
  (switch Utilities|FlowControl|Switch|SwitchonrequestType _output_get
    (:NewEnumerator2
      (CallFunction|CreateLoginRequest)
      (EventDispatchers|AssignOnRequestComplete (Variables|Default|GetsentRequest) (delegate Custom|onRequestComplete) :!label _label))
    (:NewEnumerator3
      (CallFunction|CreateRegistrationRequest)
      (goto _label))
    (:NewEnumerator4
      (CallFunction|CreateActivationRequest)
      (goto _label))
    (:NewEnumerator7
      (CallFunction|CreateLoadProfileRequest)
      (goto _label))
    (:NewEnumerator5
      (CallFunction|CreateServerRequest)
      (Development|PrintString "SERVER REQUEST COMPLETE"))))

(fn ConstructionScript)

(fn CreateLoginRequest
  (bind _mygameinstanceref (Utilities|GetGameInstance))
  (bind _mygameinstanceref_2 (Utilities|GetGameInstance))
  (bind _loginwidgetref (Variables|/Game/Blueprints/gameStructure/myGameInstance.myGameInstance_C|GetloginWidgetRef _mygameinstanceref_2))
  (bind _loginwidgetref_2 (Variables|/Game/Blueprints/gameStructure/myGameInstance.myGameInstance_C|GetloginWidgetRef _mygameinstanceref))
  (bind _returnvalue (Class|VaRestRequestJSON|GetRequestObject (Variables|Default|GetsentRequest)))
  (LocalVariables|SetloginRequestObject _returnvalue)
  (Class|VaRestJsonObject|SetStringField (LocalVariables|GetloginRequestObject) "login" (Utilities|String|ToString(Text) (Class|EditableTextBox|GetText (Variables|/Game/Blueprints/widget/loginWidget.loginWidget_C|GetloginAccountNameField _loginwidgetref))))
  (Class|VaRestJsonObject|SetStringField (LocalVariables|GetloginRequestObject) "password" (Utilities|String|ToString(Text) (Class|EditableTextBox|GetText (Variables|/Game/Blueprints/widget/loginWidget.loginWidget_C|GetloginPasswordField _loginwidgetref))))
  (Rendering|Components|TextRender|SetText (Variables|/Game/Blueprints/widget/loginWidget.loginWidget_C|GetloginAccountNameField _loginwidgetref_2) "")
  (Rendering|Components|TextRender|SetText (Variables|/Game/Blueprints/widget/loginWidget.loginWidget_C|GetloginPasswordField _loginwidgetref_2) "")
  (CallFunction|CallPhpScript (Variables|Default|GetsentRequest) "login"))

(fn CallPhpScript
  (params (request :type Va%20Rest%20Request%20JSON%20Object%20Reference) (php%20Script%20Name :type String))
  (bind _mygameinstanceref (Utilities|GetGameInstance))
  (bind _hostname (Variables|/Game/Blueprints/gameStructure/myGameInstance.myGameInstance_C|GethostName _mygameinstanceref))
  (bind _returnvalue (Utilities|String|EndsWith _hostname "/"))
  (bind _returnvalue_2 (Utilities|String|Append _hostname "/"))
  (bind _returnvalue_3 (select _returnvalue _hostname _returnvalue_2))
  (bind _returnvalue_4 (Utilities|String|Append _returnvalue_3 php%20Script%20Name))
  (bind _returnvalue_5 (Utilities|String|Append _returnvalue_4 ".php"))
  (Development|PrintString _returnvalue_5)
  (Class|VaRestRequestJSON|ProcessURL request _returnvalue_5))

(fn CreateRegistrationRequest
  (bind _returnvalue (Class|VaRestRequestJSON|GetRequestObject (Variables|Default|GetsentRequest)))
  (LocalVariables|SetregistrationRequestObject _returnvalue)
  (Class|VaRestJsonObject|SetStringField (LocalVariables|GetregistrationRequestObject) "accountname" (Utilities|String|ToString(Text) (Class|EditableTextBox|GetText (Variables|/Game/Blueprints/widget/loginWidget.loginWidget_C|GetregistrationAccountNameField (Variables|/Game/Blueprints/gameStructure/myGameInstance.myGameInstance_C|GetloginWidgetRef (Utilities|GetGameInstance))))))
  (Class|VaRestJsonObject|SetStringField (LocalVariables|GetregistrationRequestObject) "accountemail" (Utilities|String|ToString(Text) (Class|EditableTextBox|GetText (Variables|/Game/Blueprints/widget/loginWidget.loginWidget_C|GetregistrationEmailField (Variables|/Game/Blueprints/gameStructure/myGameInstance.myGameInstance_C|GetloginWidgetRef (Utilities|GetGameInstance))))))
  (Class|VaRestJsonObject|SetStringField (LocalVariables|GetregistrationRequestObject) "accountpassword" (Utilities|String|ToString(Text) (Class|EditableTextBox|GetText (Variables|/Game/Blueprints/widget/loginWidget.loginWidget_C|GetregistrationPasswordField (Variables|/Game/Blueprints/gameStructure/myGameInstance.myGameInstance_C|GetloginWidgetRef (Utilities|GetGameInstance))))))
  (Class|VaRestJsonObject|SetStringField (LocalVariables|GetregistrationRequestObject) "accountsecurityquestion" (Class|ComboBoxString|GetSelectedOption (Variables|/Game/Blueprints/widget/loginWidget.loginWidget_C|GetRegistrationSecurityQuestions (Variables|/Game/Blueprints/gameStructure/myGameInstance.myGameInstance_C|GetloginWidgetRef (Utilities|GetGameInstance)))))
  (Class|VaRestJsonObject|SetStringField (LocalVariables|GetregistrationRequestObject) "accountsecurityanswer" (Utilities|String|ToString(Text) (Class|EditableTextBox|GetText (Variables|/Game/Blueprints/widget/loginWidget.loginWidget_C|GetregistrationSecurityAnswerField (Variables|/Game/Blueprints/gameStructure/myGameInstance.myGameInstance_C|GetloginWidgetRef (Utilities|GetGameInstance))))))
  ;[0.2359 0.6483 1] create a random 8 letter string
  (for _index (range 0 8)
    (Variables|Default|SetrandomAccString (Utilities|String|Append (Utilities|Array|Get(acopy) (Variables|Default|GetalphabetArray) (Math|Random|RandomInteger 52)) (Variables|Default|GetrandomAccString)))
    ;[0.2359 0.6483 1] create a random number between 0 and 99999
    (Variables|Default|SetrandomAccNumber (Utilities|String|ToString(Integer) (Math|Random|RandomInteger 99999))))
  ;[0.2359 0.6483 1] create the random accountUniqueID by combining the random string and random number
  (bind _output_get (Variables|Default|SetaccountUniqueID (Utilities|String|Append (Variables|Default|GetrandomAccNumber) (Variables|Default|GetrandomAccString))))
  ;[0.2359 0.6483 1] turn the random accountUniqueID into a char array
  (bind _output_get_2 (Variables|Default|SetuniqueCharArray (Utilities|String|GetCharacterArrayfromString _output_get)))
  ;[0.2359 0.6483 1] loop through the char array and pick a char at random then add it back to the accountUniqueId string so now we have a completly random unique id with letters and numbers mixed together
  (for _index_2 (range 0 5)
    (bind _output_get_3 (Variables|Default|SetaccountUniqueID (Utilities|String|Append (Variables|Default|GetaccountUniqueID) (Utilities|Array|Get(acopy) _output_get_2 (Math|Random|RandomInteger (Utilities|Array|Length _output_get_2)))))))
  (Class|VaRestJsonObject|SetStringField (LocalVariables|GetregistrationRequestObject) "accountuniqueID" _output_get_3)
  (Rendering|Components|TextRender|SetText (Variables|/Game/Blueprints/widget/loginWidget.loginWidget_C|GetregistrationAccountNameField (Variables|/Game/Blueprints/gameStructure/myGameInstance.myGameInstance_C|GetloginWidgetRef (Utilities|GetGameInstance))) "")
  (Rendering|Components|TextRender|SetText (Variables|/Game/Blueprints/widget/loginWidget.loginWidget_C|GetregistrationEmailField (Variables|/Game/Blueprints/gameStructure/myGameInstance.myGameInstance_C|GetloginWidgetRef (Utilities|GetGameInstance))) "")
  (Rendering|Components|TextRender|SetText (Variables|/Game/Blueprints/widget/loginWidget.loginWidget_C|GetregistrationPasswordField (Variables|/Game/Blueprints/gameStructure/myGameInstance.myGameInstance_C|GetloginWidgetRef (Utilities|GetGameInstance))) "")
  (Rendering|Components|TextRender|SetText (Variables|/Game/Blueprints/widget/loginWidget.loginWidget_C|GetregistrationSecurityAnswerField (Variables|/Game/Blueprints/gameStructure/myGameInstance.myGameInstance_C|GetloginWidgetRef (Utilities|GetGameInstance))) "")
  (CallFunction|CallPhpScript (Variables|Default|GetsentRequest) "registration"))

(fn OnResponceRegistration
  (bind _mygameinstanceref (Utilities|GetGameInstance))
  (bind _loginwidgetref (Variables|/Game/Blueprints/gameStructure/myGameInstance.myGameInstance_C|GetloginWidgetRef _mygameinstanceref))
  (bind _returnvalue (Class|VaRestRequestJSON|GetResponseObject (Variables|Default|GetsentRequest)))
  (LocalVariables|SetregistrationResponceObject _returnvalue)
  (if (Utilities|Enum|Equal(Enum) (Class|VaRestJsonObject|GetStringField _returnvalue "status") "OK")
    (Default|DisplayErrorMessage _loginwidgetref "Registration Succesfull")
    (Default|GotoActivationPanel _loginwidgetref)
    (else
      (Default|DisplayErrorMessage (Variables|/Game/Blueprints/gameStructure/myGameInstance.myGameInstance_C|GetloginWidgetRef (Utilities|GetGameInstance)) (Utilities|Text|ToText(String) (Class|VaRestJsonObject|GetStringField _returnvalue "status"))))))

(fn CreateServerRequest
  (CallFunction|CallPhpScript (Variables|Default|GetsentRequest) "sendStartServerRequest"))

(fn CreateShutdownServerRequest
  (CallFunction|CallPhpScript (Variables|Default|GetsentRequest) "sendStartServerRequest"))

(fn OnResponceLogin
  (bind _mygameinstanceref (Utilities|GetGameInstance))
  (bind _returnvalue (Class|VaRestRequestJSON|GetResponseObject (Variables|Default|GetsentRequest)))
  (LocalVariables|SetloginResponceObject _returnvalue)
  (if (Utilities|Enum|Equal(Enum) (Class|VaRestJsonObject|GetStringField _returnvalue "status") "OK")
    (Default|DisplayErrorMessage (Variables|/Game/Blueprints/gameStructure/myGameInstance.myGameInstance_C|GetloginWidgetRef (Utilities|GetGameInstance)) "Log in Succesfull")
    (Variables|/Game/Blueprints/gameStructure/myGameInstance.myGameInstance_C|SetmySessionKey _mygameinstanceref (Class|VaRestJsonObject|GetStringField (LocalVariables|GetloginResponceObject) "sessionKey"))
    (Variables|/Game/Blueprints/gameStructure/myGameInstance.myGameInstance_C|SetmyUserID _mygameinstanceref (Math|Float|Floor (Class|VaRestJsonObject|GetNumberField (LocalVariables|GetloginResponceObject) "userid")))
    (CallFunction|SendRequest "NewEnumerator7")
    (else
      (Default|DisplayErrorMessage (Variables|/Game/Blueprints/gameStructure/myGameInstance.myGameInstance_C|GetloginWidgetRef (Utilities|GetGameInstance)) (Utilities|Text|ToText(String) (Class|VaRestJsonObject|GetStringField _returnvalue "status"))))))

(fn CreateActivationRequest
  (bind _mygameinstanceref (Utilities|GetGameInstance))
  (bind _loginwidgetref (Variables|/Game/Blueprints/gameStructure/myGameInstance.myGameInstance_C|GetloginWidgetRef _mygameinstanceref))
  (bind _accountuniqueidfield (Variables|/Game/Blueprints/widget/loginWidget.loginWidget_C|GetaccountUniqueIDfield _loginwidgetref))
  (bind _returnvalue (Class|VaRestRequestJSON|GetRequestObject (Variables|Default|GetsentRequest)))
  (LocalVariables|SetregistrationRequestObject _returnvalue)
  (Class|VaRestJsonObject|SetStringField (LocalVariables|GetregistrationRequestObject) "accountUniqueID" (Utilities|String|ToString(Text) (Class|EditableTextBox|GetText _accountuniqueidfield)))
  (Rendering|Components|TextRender|SetText _accountuniqueidfield "")
  (Rendering|Components|TextRender|SetText (Variables|/Game/Blueprints/widget/loginWidget.loginWidget_C|GetaccountUniqueIDfield (Variables|/Game/Blueprints/gameStructure/myGameInstance.myGameInstance_C|GetloginWidgetRef (Utilities|GetGameInstance))) "")
  (CallFunction|CallPhpScript (Variables|Default|GetsentRequest) "activationRequest"))

(fn OnResponceActivation
  (bind _mygameinstanceref (Utilities|GetGameInstance))
  (bind _loginwidgetref (Variables|/Game/Blueprints/gameStructure/myGameInstance.myGameInstance_C|GetloginWidgetRef _mygameinstanceref))
  (bind _returnvalue (Class|VaRestRequestJSON|GetResponseObject (Variables|Default|GetsentRequest)))
  (LocalVariables|SetactivationResponceObject _returnvalue)
  (if (Utilities|Enum|Equal(Enum) (Class|VaRestJsonObject|GetStringField _returnvalue "status") "account found")
    (Default|DisplayErrorMessage _loginwidgetref "ACCOUNT FOUND")
    (Default|GotoLoginPanelfromActivation _loginwidgetref)
    (else
      (Default|DisplayErrorMessage (Variables|/Game/Blueprints/gameStructure/myGameInstance.myGameInstance_C|GetloginWidgetRef (Utilities|GetGameInstance)) (Utilities|Text|ToText(String) (Class|VaRestJsonObject|GetStringField _returnvalue "status"))))))

(fn CreateLoadProfileRequest
  (bind _mygameinstanceref (Utilities|GetGameInstance))
  (bind _returnvalue (Class|VaRestRequestJSON|GetRequestObject (Variables|Default|GetsentRequest)))
  (LocalVariables|SetloadProfileRequestObject _returnvalue)
  (Class|VaRestJsonObject|SetStringField (LocalVariables|GetloadProfileRequestObject) "sessionkey" (Variables|/Game/Blueprints/gameStructure/myGameInstance.myGameInstance_C|GetmySessionKey _mygameinstanceref))
  (Class|VaRestJsonObject|SetNumberField (LocalVariables|GetloadProfileRequestObject) "userid" (Math|Conversions|ToFloat(Integer) (Variables|/Game/Blueprints/gameStructure/myGameInstance.myGameInstance_C|GetmyUserID _mygameinstanceref)))
  (CallFunction|CallPhpScript (Variables|Default|GetsentRequest) "loadprofile"))

(fn OnResponseLoadProfile
  (bind _returnvalue (Class|VaRestRequestJSON|GetResponseObject (Variables|Default|GetsentRequest)))
  (bind _output_get (LocalVariables|SetloadProfileResponceObject _returnvalue))
  (if (Utilities|Enum|Equal(Enum) (Class|VaRestJsonObject|GetStringField _output_get "status") "Ok")
    ;[0.2359 0.6483 1] check that we have loaded a profile
    (bind _returnvalue_2 (Class|VaRestJsonObject|GetObjectArrayField (LocalVariables|GetloadProfileResponceObject) "profile"))
    (if true
      (for _array_element _returnvalue_2
        (Variables|Default|SetcurrentProfileObject _array_element))
      (Default|EnterLobbyLevel (Utilities|GetGameInstance))
      (else
        (Development|PrintString "error profile not loaded")))
    (else
      (Default|DisplayErrorMessage (Variables|/Game/Blueprints/gameStructure/myGameInstance.myGameInstance_C|GetloginWidgetRef (Utilities|GetGameInstance)) (Utilities|Text|ToText(String) (Class|VaRestJsonObject|GetStringField _output_get "status"))))))